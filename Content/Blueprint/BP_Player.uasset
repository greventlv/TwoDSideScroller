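; Player character for a 2D side-view game, with flipbook animation, jumping, climbing, shooting and a charge move.
; Input handles movement, facing, camera projection toggle and BP_Shot spawning, while Tick overrides the speed-based idle/run flipbook according to State.
; Damage, also triggered by a debug-style key, ignores DamageIn for a fixed health loss, then sets Dead or applies knockback and a looping blink timer.
; BeginPlay creates the HUD widget.
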(event Custom|Blink
  (bind _sprite (Variables|Default|GetSprite))
  ;[1 1 1] DamageSystem
  (Development|SetHiddeninGame _sprite true false)
  (Utilities|FlowControl|Delay 0.1)
  (Development|SetHiddeninGame _sprite false false))

(event Custom|DamageSystem
  (params (DamageIn :type Float%20%28single-precision%29))
  ;[1 1 1] DamageSystem
  (Variables|Default|SetIsHit true)
  (bind _output_get (Variables|Default|SetHealthCurrent (- (Variables|Default|GetHealthCurrent) 0.19)))
  (if (<= _output_get 0.0)
    (Variables|Default|SetState "NewEnumerator5")
    (else
      (Variables|Default|SetState "NewEnumerator4")
      (Physics|AddForce (Variables|Character|GetCharacterMovement) (Math|Vector|MakeVector (* (Variables|Default|GetFacing) (Variables|Default|GetKnockBack)) 0.0 2e+06))
      (Utilities|Time|SetTimerbyFunctionName 0 "Blink" 2.0 true))))

(event Custom|UpdateAnimation
  ;[1 1 1] Handle Animation
  (Sprite|SetFlipbook (Variables|Default|GetSprite) (select (> (Math|Vector|VectorLength (Transformation|GetVelocity)) 0.0) "/Game/Sprites/Character/Anim_Run.Anim_Run" "/Game/Sprites/Character/Anim_IdleStanding.Anim_IdleStanding")))

(event EventOnLanded
  (params (Hit :type Hit%20Result%20Structure%20%28by%20ref%29))
  ;[1 1 1] Handle Jump
  (if (Variables|Default|GetIsHit)
    (Variables|Default|SetState "NewEnumerator0")
    (CallFunction|UpdateAnimation)
    (Utilities|FlowControl|Delay 0.25)
    (Variables|Default|SetIsHit false)
    (CallFunction|UpdateAnimation)
    (else
      (Variables|Default|SetState "NewEnumerator0")
      (CallFunction|UpdateAnimation))))

(event EventTick
  (params (DeltaSeconds :type Float%20%28single-precision%29))
  (bind _sprite (Variables|Default|GetSprite))
  ;[1 0.5938 0.5938] Tick - Updates animation
  (CallFunction|UpdateAnimation)
  (switch Utilities|FlowControl|Switch|SwitchonBP_PlayerState (Variables|Default|GetState)
    (:NewEnumerator1
      (Math|Float|CompareFloat (.X (Math|Vector|BreakVector (Variables|/Script/Engine.MovementComponent|GetVelocity (Pawn|GetMovementComponent)))) 0.0
        (:>
          (Pawn|SetControlRotation (Pawn|GetController) (Math|Rotator|MakeRotator 0.0 0.0 0.0) :!label _label)
          (Variables|Default|SetState "NewEnumerator1"))
        (:==
          (if (Variables|Default|GetbisMovingRight)
            (goto _label)
            (else
              (Pawn|SetControlRotation (Pawn|GetController) (Math|Rotator|MakeRotator 0.0 0.0 1.8e+02) :!label _label_2)
              (Variables|Default|SetState "NewEnumerator1"))))
        (:<
          (goto _label_2))))
    (:NewEnumerator2
      (Sprite|SetFlipbook _sprite "/Game/Sprites/Character/Anim_Jump.Anim_Jump"))
    (:NewEnumerator4
      (Sprite|SetFlipbook _sprite "/Game/Sprites/Character/Anim_Hit.Anim_Hit"))
    (:NewEnumerator8
      (Sprite|SetFlipbook _sprite "/Game/Sprites/Character/Anim_Sitting.Anim_Sitting"))
    (:NewEnumerator5
      (Sprite|SetFlipbook _sprite "/Game/Sprites/Character/Anim_Dead.Anim_Dead"))
    (:NewEnumerator6
      (Sprite|SetFlipbook (Variables|Default|GetSprite) "/Game/Sprites/Character/Anim_Makanke.Anim_Makanke")
      (Audio|PlaySound2D "/Game/Audio/Final_Flash_Charge_Sound_Effect_DBZ.Final_Flash_Charge_Sound_Effect_DBZ" 0.1 1.0 0.0 0 0)
      (Utilities|FlowControl|Delay 0.2))
    (:NewEnumerator9
      (Sprite|SetFlipbook (Variables|Default|GetSprite) "/Game/Sprites/Character/Anim_ShootingStanding.Anim_ShootingStanding"))))

(event EventBeginPlay
  ;[1 0.5312 0.5312] Initialize
  (Utilities|FlowControl|Sequence
    (:then_0
      (Class|ActorComponent|SetIsReplicated (Variables|Default|GetSprite) true))
    (:then_1
      (bind _returnvalue (UserInterface|CreateWidget "/Game/Blueprint/BPW_HUD.BPW_HUD_C" (Game|GetPlayerController 0)))
      (bind _output_get (Variables|Default|SetHealthBar _returnvalue))
      (UserInterface|Viewport|AddtoViewport _output_get 0))))

(event Input|ActionEvents|InputActionMakenk
  (params (Key :type Key%20Structure))
  ;[1 1 1] Fighting
  (:Pressed
    (Variables|Default|SetState "NewEnumerator6")))

(event Input|ActionEvents|InputActionEscapeQuit
  (params (Key :type Key%20Structure))
  (:Released
    (Game|QuitGame 0 "Quit" false)))

(event Input|ActionEvents|InputActionShoot
  (params (Key :type Key%20Structure))
  ;[1 1 1] Fighting
  (:Pressed
    (Game|SpawnActorfromClass "/Game/Blueprint/BP_Shot.BP_Shot_C" (Transformation|GetWorldTransform (Variables|Default|GetArrowComponent)) "AdjustIfPossibleButAlwaysSpawn" 0 0)
    (Variables|Default|SetState "NewEnumerator9")
    (CallFunction|UpdateAnimation :!label _label))
  (:Released
    (Utilities|FlowControl|RetriggerableDelay 0.2)
    (Variables|Default|SetState "NewEnumerator0")
    (goto _label)))

(event Input|ActionEvents|InputActionChangePOV
  (params (Key :type Key%20Structure))
  (bind _sideviewcameracomponent (Variables|Camera|GetSideViewCameraComponent))
  (:Pressed
    (Utilities|FlowControl|FlipFlop
      (:A
        (Class|CameraComponent|SetProjectionMode _sideviewcameracomponent "Orthographic"))
      (:B
        (Class|CameraComponent|SetProjectionMode _sideviewcameracomponent "Perspective")))))

(event Input|ActionEvents|InputActionJump
  (params (Key :type Key%20Structure))
  (bind _climbspeed (Variables|Default|GetClimbSpeed))
  (bind _returnvalue (* 1.0 _climbspeed))
  ;[1 1 1] Handle Jump
  (:Pressed
    (if (Variables|Default|GetCanClimb)
      (Development|PrintString (Utilities|String|ToString(Float) _returnvalue))
      (Transformation|AddActorLocalOffset (Math|Vector|MakeVector 0.0 0.0 _returnvalue) false false)
      (else
        (Audio|PlaySound2D "/Game/Audio/Mario-jump-sound.Mario-jump-sound" 0.1 1.0 0.0 0 0)
        (Character|Jump)
        (Variables|Default|SetState "NewEnumerator2"))))
  (:Released
    (Character|StopJumping)))

(event Input|AxisEvents|InputAxisMoveUp
  (params (AxisValue :type Float%20%28single-precision%29))
  ;[1 1 1] Handle Jump
)

(event Input|AxisEvents|InputAxisMoveRight
  (params (AxisValue :type Float%20%28single-precision%29))
  ;[1 1 1] Handle movement
  (Pawn|Input|AddMovementInput "1.000000, 0, 0" AxisValue false)
  (CallFunction|UpdateAnimation)
  (Math|Float|CompareFloat AxisValue 0.0
    (:>
      (Pawn|SetControlRotation (Pawn|GetController) (Math|Rotator|MakeRotator 0.0 0.0 0.0))
      (Variables|Default|SetFacing 1))
    (:<
      (Pawn|SetControlRotation (Pawn|GetController) (Math|Rotator|MakeRotator 0.0 0.0 1.8e+02))
      (Variables|Default|SetFacing -1))))

(event Input|KeyboardEvents|1
  (params (Key :type Key%20Structure))
  ;[1 1 1] DamageSystem
  (:Pressed
    (Variables|Default|SetIsHit true)
    (bind _output_get (Variables|Default|SetHealthCurrent (- (Variables|Default|GetHealthCurrent) 0.19)))
    (if (<= _output_get 0.0)
      (Variables|Default|SetState "NewEnumerator5")
      (else
        (Variables|Default|SetState "NewEnumerator4")
        (Physics|AddForce (Variables|Character|GetCharacterMovement) (Math|Vector|MakeVector (* (Variables|Default|GetFacing) (Variables|Default|GetKnockBack)) 0.0 2e+06))
        (Utilities|Time|SetTimerbyFunctionName 0 "Blink" 2.0 true)))))

(event Input|TouchEvents|InputTouch
  (params (Location :type Vector) (FingerIndex :type ETouchIndex%20Enum))
  ;[1 1 1] Handle Jump
  (:Pressed
    (Audio|PlaySound2D "/Game/Audio/Mario-jump-sound.Mario-jump-sound" 0.1 1.0 0.0 0 0)
    (Character|Jump)
    (Variables|Default|SetState "NewEnumerator2"))
  (:Released
    (Character|StopJumping)))

(fn ConstructionScript)